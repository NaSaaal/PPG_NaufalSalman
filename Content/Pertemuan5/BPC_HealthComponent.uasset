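; BPC_HealthComponent is a health component that sets Health to MaxHealth on BeginPlay and exposes a TakeDamage function.
; TakeDamage compares Health minus Damage against MaxHealth, resetting Health to the maximum when the result reaches or exceeds it.
; Otherwise it assigns Health to itself, so the damage is never subtracted, then calls OnDeath if Health is zero or below.
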(event EventBeginPlay
  (Variables|Default|SetHealth (Variables|Default|GetMaxHealth)))

(event EventTick
  (params (DeltaSeconds :type Float%20%28single-precision%29)))

(fn TakeDamage
  (params (Damage :type Float%20%28double-precision%29))
  (bind _maxhealth (Variables|Default|GetMaxHealth))
  (if (< (- (Variables|Default|GetHealth) Damage) _maxhealth)
    (bind _output_get (Variables|Default|SetHealth (Variables|Default|GetHealth)))
    (if (<= _output_get 0.0)
      (Default|CallOnDeath))
    (else
      (Variables|Default|SetHealth _maxhealth))))